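; Power-up pickup that enables the powered attack on the player who overlaps it.
; A Bounce timeline animates the plane's height while the actor spins each tick, and the box's collision stays off until a one-second delay after spawn.
; On overlap with Player_BP it sets PoweredAttackEnabled, destroys itself and shows HeavyAttack on its own Player_HUD instance, created at BeginPlay and not added to the viewport here.
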(event `self.ReceiveBeginPlay`
  (bind _returnvalue (`|CreateWidget` "/Game/UI/Player_HUD.Player_HUD_C"))
  (set `self.PlayerHUD` _returnvalue)
  (`PrimitiveComponent.SetCollisionEnabled` (`self.Box`) "NoCollision")
  (bind (_direction _baunss) (`Timeline|Bounce` :!via `PlayFromStart`)
    (:`Update`
      (`SceneComponent.K2_SetRelativeLocation` (`self.Plane`) (`KismetMathLibrary.MakeVector` 0.0 0.0 _baunss) false false)
      (`KismetSystemLibrary.Delay` 1.0)
      (`PrimitiveComponent.SetCollisionEnabled` (`self.Box`) "QueryAndPhysics"))))

(event `self.ReceiveTick`
  (params (DeltaSeconds :type "Float (single-precision)"))
  (`self.K2_AddActorLocalRotation` (`KismetMathLibrary.MakeRotator` 0.0 0.0 2.0)))

(event `self.Box.OnComponentBeginOverlap`
  (params (OverlappedComponent :type "PrimitiveComponent Object Reference") (OtherActor :type "Actor Object Reference") (OtherComp :type "PrimitiveComponent Object Reference") (OtherBodyIndex :type Integer) (bFromSweep :type Boolean) (SweepResult :type "HitResult Structure (by ref)"))
  (bind _asplayer_bp (cast `/Game/Yilva/Player_BP` OtherActor))
  (set `/Game/Yilva/Player_BP.PoweredAttackEnabled` true _asplayer_bp)
  (`self.K2_DestroyActor`)
  (`Widget.SetVisibility` (`/Game/UI/Player_HUD.HeavyAttack` (`self.PlayerHUD`)) "Visible"))

(fn `UserConstructionScript`)