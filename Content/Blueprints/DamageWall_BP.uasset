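; DamageWall_BP is a wall that damages the player on contact unless whisp form is active, which lets them pass through.
; Every tick, BlockBox ignores pawns while WhispFormNiagara is active, and otherwise restores blocking only if it overlaps the player.
; Box overlap applies damage unless the player is phasing, immune or dead.
; It then briefly toggles its Pawn response off and back to Overlap, intended to retrigger hits after immunity ends.
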(event `self.ReceiveTick`
  (params (DeltaSeconds :type "Float (single-precision)"))
  ;[1 1 1] WhispFormCheck
  (bind _asplayer_bp (cast `/Game/Yilva/Player_BP` (`GameplayStatics.GetPlayerCharacter` 0)))
  (if (`ActorComponent.IsActive` (`/Game/Yilva/Player_BP.WhispForm_Niagara` _asplayer_bp))
    (`PrimitiveComponent.SetCollisionResponseToChannel` (`self.BlockBox`) "ECC_Pawn" "ECR_Ignore")
    (elif (`PrimitiveComponent.IsOverlappingActor` (`self.BlockBox`) _asplayer_bp)
      (`PrimitiveComponent.SetCollisionResponseToChannel` (`self.BlockBox`) "ECC_Pawn" "ECR_Block"))))

(event `self.Box.OnComponentBeginOverlap`
  (params (OverlappedComponent :type "PrimitiveComponent Object Reference") (OtherActor :type "Actor Object Reference") (OtherComp :type "PrimitiveComponent Object Reference") (OtherBodyIndex :type Integer) (bFromSweep :type Boolean) (SweepResult :type "HitResult Structure (by ref)"))
  (bind _asplayer_bp (cast `/Game/Yilva/Player_BP` OtherActor))
  (if (`ActorComponent.IsActive` (`/Game/Yilva/Player_BP.WhispForm_Niagara` _asplayer_bp))
    _
    (elif (`/Game/Yilva/Player_BP.IsImmune` _asplayer_bp)
      _
      (elif (not (`/Game/Yilva/Player_BP.Died` _asplayer_bp))
        (`GameplayStatics.ApplyDamage` OtherActor 0.33)
        ;[1 1 1] Make player get hit again when immunity disappears
        (`PrimitiveComponent.SetCollisionResponseToChannel` (`self.Box`) "ECC_Pawn" "ECR_Ignore")
        (`KismetSystemLibrary.Delay` 0.2)
        (`PrimitiveComponent.SetCollisionResponseToChannel` (`self.Box`) "ECC_Pawn" "ECR_Overlap")))))

(fn `UserConstructionScript`)