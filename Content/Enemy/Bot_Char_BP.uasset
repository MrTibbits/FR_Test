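; Enemy bot character Blueprint that drops a power attack power-up when it takes damage.
; Any damage spawns PowerAttack_PowerUp_BP at the ItemLocation transform, turns off capsule collision, then destroys the bot after a short delay, with no health check.
; Tick spins the BotTorus component on roll and yaw by a fixed step each frame, independent of delta time.
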(event `self.ReceiveAnyDamage`
  (params (Damage :type "Float (single-precision)") (DamageType :type "DamageType Object Reference") (InstigatedBy :type "Controller Object Reference") (DamageCauser :type "Actor Object Reference"))
  (`|SpawnActorFromClass` "/Game/Blueprints/PowerAttack_PowerUp_BP.PowerAttack_PowerUp_BP_C" (`SceneComponent.K2_GetComponentToWorld` (`self.ItemLocation`)) "Undefined" "OverrideRootScale" null null)
  (`PrimitiveComponent.SetCollisionEnabled` (`self.CapsuleComponent`) "NoCollision")
  (`KismetSystemLibrary.Delay` 0.2)
  (`self.K2_DestroyActor`))

(event `self.ReceiveTick`
  (params (DeltaSeconds :type "Float (single-precision)"))
  (`SceneComponent.K2_AddLocalRotation` (`self.BotTorus`) (`KismetMathLibrary.MakeRotator` 2.0 0.0 2.0) false false))

(fn `UserConstructionScript`)